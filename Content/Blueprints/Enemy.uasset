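; Cyclops enemy that chases the player character, takes damage and dies.
; PawnSensing sightings of a Character_Blueprint trigger AIMoveTo toward it.
; AnyDamage lowers Health and switches on RandomInteger(1), which always yields 0, so only the first of two hit montages is reached.
; Health is checked when the montage completes; at zero or below it plays the death animation, sets IfDead and destroys the actor after a delay.
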(event `self.ReceiveAnyDamage`
  (params (Damage :type "Float (single-precision)") (DamageType :type "DamageType Object Reference") (InstigatedBy :type "Controller Object Reference") (DamageCauser :type "Actor Object Reference"))
  ;[1 1 1] Damage/Health System
  (if (not (`self.IfDead`))
    (`KismetSystemLibrary.PrintString` (`KismetStringLibrary.Conv_DoubleToString` Damage))
    (bind _output_get (set `self.Health` (- (`self.Health`) Damage)))
    (switch `int` (`KismetMathLibrary.RandomInteger` 1)
      (:`0`
        (`|PlayMontage` (`self.SkeletalMesh`) "/Game/ma12_Monsterset_04/PolyHP_Cyclops/Animations/Cyclops_Damage_01.Cyclops_Damage_01"
          (:`OnCompleted`
            _)))
      (:`1`
        (`|PlayMontage` null "/Game/ma12_Monsterset_04/PolyHP_Cyclops/Animations/Cyclops_Damage_02.Cyclops_Damage_02"
          (:`OnCompleted`
            _))))
    (if (<= _output_get 0.0)
      (`SkeletalMeshComponent.PlayAnimation` (`self.SkeletalMesh`) "/Game/ma12_Monsterset_04/PolyHP_Cyclops/Animations/ms04_02_Die.ms04_02_Die" false)
      (set `self.IfDead` true)
      (`KismetSystemLibrary.Delay` 2.0)
      (`self.K2_DestroyActor`))))

(event `self.PawnSensing.OnSeePawn`
  (params (Pawn :type "Pawn Object Reference"))
  (bind _ascharacter_blueprint (cast `/Game/Character/Blueprints/Character_Blueprint` Pawn))
  (`|AIMoveTo` self (0.0 0.0 0.0) _ascharacter_blueprint))

(fn `UserConstructionScript`)