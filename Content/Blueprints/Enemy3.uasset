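; Enemy3 is a cyclops enemy that takes damage and dies.
; AnyDamage lowers Health and plays a hit montage (the random pick always yields the first), then at zero Health plays a death animation and destroys the actor after a delay.
; Box overlap begin and end toggle its Widget's visibility.
; Pawn-sensing chase logic is disconnected, and the BeginPlay EnemyUI2 lookup does nothing with its result.
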(event `self.PawnSensing.OnSeePawn`
  (params (Pawn :type "Pawn Object Reference")))

(event `self.ReceiveBeginPlay`
  (bind _foundwidgets (`WidgetBlueprintLibrary.GetAllWidgetsOfClass` "/Game/UI/EnemyUI2.EnemyUI2_C"))
  (for _array_element _foundwidgets
    _)
  (cast `/Game/UI/EnemyUI2` _array_element))

(event `self.Box.OnComponentBeginOverlap`
  (params (OverlappedComponent :type "PrimitiveComponent Object Reference") (OtherActor :type "Actor Object Reference") (OtherComp :type "PrimitiveComponent Object Reference") (OtherBodyIndex :type Integer) (bFromSweep :type Boolean) (SweepResult :type "HitResult Structure (by ref)"))
  (`SceneComponent.ToggleVisibility` (`self.Widget`) false))

(event `self.Box.OnComponentEndOverlap`
  (params (OverlappedComponent :type "PrimitiveComponent Object Reference") (OtherActor :type "Actor Object Reference") (OtherComp :type "PrimitiveComponent Object Reference") (OtherBodyIndex :type Integer))
  (`SceneComponent.ToggleVisibility` (`self.Widget`) false))

(event `self.ReceiveAnyDamage`
  (params (Damage :type "Float (single-precision)") (DamageType :type "DamageType Object Reference") (InstigatedBy :type "Controller Object Reference") (DamageCauser :type "Actor Object Reference"))
  (bind _mesh (`self.Mesh`))
  (if (not (`self.IsDead`))
    (`KismetSystemLibrary.PrintString` (`KismetStringLibrary.Conv_DoubleToString` Damage))
    (bind _output_get (set `self.Health` (- (`self.Health`) Damage)))
    (switch `int` (`KismetMathLibrary.RandomInteger` 1)
      (:`0`
        (`|PlayMontage` _mesh "/Game/ma12_Monsterset_04/PolyHP_Cyclops/Animations/Cyclops_Damage_01.Cyclops_Damage_01"
          (:`OnCompleted`
            _)
          (:`OnInterrupted`
            _)))
      (:`1`
        (`|PlayMontage` _mesh "/Game/ma12_Monsterset_04/PolyHP_Cyclops/Animations/Cyclops_Damage_02.Cyclops_Damage_02"
          (:`OnCompleted`
            _)
          (:`OnInterrupted`
            _))))
    (if (<= _output_get 0.0)
      (set `self.IsDead` true)
      (`SkeletalMeshComponent.PlayAnimation` (`self.Mesh`) "/Game/ma12_Monsterset_04/PolyHP_Cyclops/Animations/ms04_02_Die.ms04_02_Die" false)
      (`KismetSystemLibrary.Delay` 2.0)
      (`self.K2_DestroyActor`))))

(fn `UserConstructionScript`)